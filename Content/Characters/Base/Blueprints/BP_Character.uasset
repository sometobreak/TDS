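; Base top-down shooter character that turns its capsule toward the mouse cursor each tick, with an adjustable boom camera.
; Mouse wheel zooms instantly or in timer-driven steps; right mouse switches aim state and slides the camera out or back.
; Space plays hip or ironsight fire montages, and step sounds follow the traced surface type.
; Sprint input runs debug prints and cursor-based move/offset calls, while the timer-driven sprint logic is disconnected.
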(event `self.ReceiveTick`
  (params (DeltaSeconds :type "Float (single-precision)"))
  (bind _returnvalue (`self.K2_GetActorLocation`))
  (bind (_worldlocation _worlddirection) (`PlayerController.DeprojectMousePositionToWorld` (`GameplayStatics.GetPlayerController` 0)))
  (bind (_returnvalue_x _returnvalue_y) (`KismetMathLibrary.BreakVector` (+ _worldlocation (* _worlddirection (`SpringArmComponent.TargetArmLength` (`self.CameraBoom`))))))
  ;[1 1 1] Event Tick
  (`SceneComponent.K2_SetWorldRotation` (`self.CapsuleComponent`) (`KismetMathLibrary.FindLookAtRotation` _returnvalue (`KismetMathLibrary.MakeVector` _returnvalue_x _returnvalue_y (.z _returnvalue))) false false))

(event `PlayStepSound`
  (bind _returnvalue (`self.K2_GetActorLocation`))
  ;[1 1 1] Step Sound
  (bind _outhit (`KismetSystemLibrary.LineTraceSingle` _returnvalue (- _returnvalue (0.0 0.0 150.0)) "TraceTypeQuery1"))
  (bind (_bblockinghit _binitialoverlap _time _distance _location _impactpoint _normal _impactnormal _physmat) (`GameplayStatics.BreakHitResult` _outhit))
  (if (`KismetSystemLibrary.IsValid` _physmat)
    (`GameplayStatics.PlaySoundAtLocation` (select `EPhysicalSurface` (`PhysicalMaterial.SurfaceType` _physmat) :`SurfaceType1` "/Game/Characters/Base/Sounds/Steps/Grass/Cue/GrassCue.GrassCue" :`SurfaceType2` "/Game/Characters/Base/Sounds/Steps/Rock/Cue/RockCue.RockCue" :`SurfaceType3` "/Game/Characters/Base/Sounds/Steps/Sand/Cue/SandCue.SandCue" :`SurfaceType4` "/Game/Characters/Base/Sounds/Steps/Wood/Cue/WoodCue.WoodCue" :!type "SoundCue Object Reference") _location (struct) 1.0 1.0 0.0 null null null)))

(event `InputAxis|MouseWheel`
  (params (AxisValue :type "Float (single-precision)"))
  (if (`self.SlideWithSmooth`)
    (`self.CameraSlideSmooth` AxisValue)
    (else
      (`self.CameraSlide` AxisValue))))

(event `Key|RightMouseButton`
  (params (Key :type "Key Structure"))
  (bind _sprintenable (`self.SprintEnable`))
  (:`Pressed`
    (if (not _sprintenable)
      (set `self.AimEnable` true)
      (`self.ChangeMovementState` "Aim_State")
      (`self.AimSlideSmooth` :!label _label)))
  (:`Released`
    (if (not _sprintenable)
      (set `self.AimEnable` false)
      (`self.ChangeMovementState` "Walk_State")
      (goto _label))))

(event `InputAction|Sprint`
  (params (Key :type "Key Structure"))
  (bind _returnvalue (`GameplayStatics.GetPlayerController` 0))
  (bind _returnvalue_2 (`self.K2_GetActorLocation`))
  (bind (_worldlocation _worlddirection) (`PlayerController.DeprojectMousePositionToWorld` _returnvalue))
  (bind _z (.z _returnvalue_2))
  (bind _y (.y _worldlocation))
  (bind _returnvalue_3 (+ (.x _worldlocation) 1000.0))
  (:`Pressed`
    (`KismetSystemLibrary.PrintString` (`KismetStringLibrary.Conv_VectorToString` _returnvalue_2))
    (`KismetSystemLibrary.PrintString` (`KismetStringLibrary.Conv_VectorToString` _worldlocation))
    (`AIBlueprintHelperLibrary.SimpleMoveToLocation` _returnvalue (`KismetMathLibrary.MakeVector` _returnvalue_3 _y _z))
    (`self.K2_AddActorWorldOffset` (`KismetMathLibrary.MakeVector` _returnvalue_3 _y _z) true)))

(event `Key|SpaceBar`
  (params (Key :type "Key Structure"))
  (bind _mesh (`self.Mesh`))
  (:`Pressed`
    (if (`self.AimEnable`)
      (`|PlayMontage` _mesh "/Game/Characters/Base/Animations/NewFire_Rifle_Ironsights_Montage.NewFire_Rifle_Ironsights_Montage")
      (else
        (`|PlayMontage` _mesh "/Game/Characters/Base/Animations/NewFire_Rifle_Hip_Montage.NewFire_Rifle_Hip_Montage")))))

(fn `AimSlideSmooth`
  (bind _returnvalue (`KismetSystemLibrary.K2_SetTimer` null "AimSlideSmoothTick" (`self.AimStepTimer`) true))
  (set `self.AimTimer` _returnvalue))

(fn `AimSlideSmoothTick`
  (bind _aimchangeslidestepdistance (`self.AimChangeSlideStepDistance`))
  (bind _heightcameramax (`self.HeightCameraMax`))
  (bind _cameraboom (`self.CameraBoom`))
  (bind _targetarmlength (`SpringArmComponent.TargetArmLength` _cameraboom))
  (if (`self.AimEnable`)
    (if (< _targetarmlength (+ _heightcameramax (`self.AimDistance`)))
      (set `SpringArmComponent.TargetArmLength` (+ _targetarmlength _aimchangeslidestepdistance) _cameraboom)
      (else
        (`KismetSystemLibrary.K2_ClearAndInvalidateTimerHandle` (`self.AimTimer`) :!label _label)))
    (elif (> _targetarmlength _heightcameramax)
      (set `SpringArmComponent.TargetArmLength` (- _targetarmlength _aimchangeslidestepdistance) _cameraboom)
      (else
        (goto _label)))))

(fn `CameraShakeEvent`
  (`GameplayStatics.PlayWorldCameraShake` "/Game/Game/Blueprints/BP_ShakeCamera.BP_ShakeCamera_C" (`SceneComponent.K2_GetComponentLocation` (`self.TopDownCameraComponent`)) 0.0 30.0))

(fn `CameraSlide`
  (params (Value :type "Float (double-precision)"))
  (bind _heightcamerachangedistance (`self.HeightCameraChangeDistance`))
  (bind _cameraboom (`self.CameraBoom`))
  (bind _targetarmlength (`SpringArmComponent.TargetArmLength` _cameraboom))
  (bind _returnvalue (- _targetarmlength _heightcamerachangedistance))
  (bind _returnvalue_2 (+ _targetarmlength _heightcamerachangedistance))
  (if (!= Value 0.0)
    (if (< Value 0.0)
      (if (>= (`self.HeightCameraMax`) _returnvalue_2)
        (set `SpringArmComponent.TargetArmLength` _returnvalue_2 _cameraboom))
      (elif (<= (`self.HeightCameraMin`) _returnvalue)
        (set `SpringArmComponent.TargetArmLength` _returnvalue _cameraboom)))))

(fn `CameraSlideSmooth`
  (params (Value :type "Float (double-precision)"))
  (bind _heightcamerachangedistance (`self.HeightCameraChangeDistance`))
  (bind _targetarmlength (`SpringArmComponent.TargetArmLength` (`self.CameraBoom`)))
  (if (`self.SlideDone`)
    (if (!= Value 0.0)
      (if (< Value 0.0)
        (if (>= (`self.HeightCameraMax`) (+ _targetarmlength _heightcamerachangedistance))
          (set `self.SlideUp` true)
          (set `self.SlideDone` false :!label _label)
          (bind _returnvalue (`KismetSystemLibrary.K2_SetTimer` null "CameraSlideSmoothTick" (`self.StepTimer`) true))
          (set `self.SlideTimer` _returnvalue))
        (elif (<= (`self.HeightCameraMin`) (- _targetarmlength _heightcamerachangedistance))
          (set `self.SlideUp` false)
          (goto _label))))))

(fn `CameraSlideSmoothTick`
  (bind _heightcamerachangeslidestepdistance (`self.HeightCameraChangeSlideStepDistance`))
  (bind _cameraboom (`self.CameraBoom`))
  (bind _targetarmlength (`SpringArmComponent.TargetArmLength` _cameraboom))
  (bind _output_get (set `self.CurrentSlideDistance` (+ (`self.CurrentSlideDistance`) _heightcamerachangeslidestepdistance)))
  (set `SpringArmComponent.TargetArmLength` (select `bool` (`self.SlideUp`) :`false` (- _targetarmlength _heightcamerachangeslidestepdistance) :`true` (+ _targetarmlength _heightcamerachangeslidestepdistance)) _cameraboom)
  (if (>= _output_get (`self.HeightCameraChangeDistance`))
    (set `self.CurrentSlideDistance` 0.0)
    (set `self.SlideDone` true)
    (`KismetSystemLibrary.K2_ClearAndInvalidateTimerHandle` (`self.SlideTimer`))))

(fn `Sprint`
  (`AIBlueprintHelperLibrary.SimpleMoveToLocation` (`GameplayStatics.GetPlayerController` 0) (+ (`self.K2_GetActorLocation`) (* (`KismetMathLibrary.Conv_RotatorToVector` (`self.K2_GetActorRotation`)) 200.0))))

(fn `UserConstructionScript`
  (bind _cameraboom (`self.CameraBoom`))
  (set `SpringArmComponent.TargetArmLength` (`self.HeightCameraMax`) _cameraboom)
  (`SceneComponent.K2_SetRelativeRotation` _cameraboom (`self.RotationCamera`) false false)
  (set `SpringArmComponent.bEnableCameraLag` (`self.Flow`) _cameraboom)
  (set `SpringArmComponent.CameraLagSpeed` (`self.CoefSmooth`) _cameraboom))