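; Top-down character Blueprint that handles aim and walk movement states, fire montages on Space, and the camera boom.
; Right mouse aims and the Walk action walks, each blocking the other, with both returning to run on release.
; Mouse wheel zooms within height limits, instantly or through looping-timer steps.
; Aiming uses a similar timer to extend the boom beyond maximum height, and a helper plays camera shake.
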(event `InputAxis|MouseWheel`
  (params (AxisValue :type "Float (single-precision)"))
  (if (`self.SlideWithSmooth`)
    (`self.CameraSlideSmooth` AxisValue)
    (else
      (`self.CameraSlide` AxisValue))))

(event `Key|RightMouseButton`
  (params (Key :type "Key Structure"))
  (bind _iswalk (`self.IsWalk`))
  (:`Pressed`
    (if (not _iswalk)
      (set `self.IsAim` true)
      (`self.ChangeMovementState` "Aim_State")
      (`self.AimSlideSmooth` :!label _label)))
  (:`Released`
    (if (not _iswalk)
      (set `self.IsAim` false)
      (`self.ChangeMovementState` "Run_State")
      (goto _label))))

(event `InputAction|Walk`
  (params (Key :type "Key Structure"))
  (bind _isaim (`self.IsAim`))
  (:`Pressed`
    (if (not _isaim)
      (set `self.IsWalk` true)
      (`self.ChangeMovementState` "Walk_State")))
  (:`Released`
    (if (not _isaim)
      (set `self.IsWalk` false)
      (`self.ChangeMovementState` "Run_State"))))

(event `Key|SpaceBar`
  (params (Key :type "Key Structure"))
  (bind _mesh (`self.Mesh`))
  (:`Pressed`
    (if (`self.IsAim`)
      (`|PlayMontage` _mesh "/Game/Blueprints/Characters/Mannequin/Animations/NewFire_Rifle_Ironsights_Montage.NewFire_Rifle_Ironsights_Montage")
      (else
        (`|PlayMontage` _mesh "/Game/Blueprints/Characters/Mannequin/Animations/NewFire_Rifle_Hip_Montage.NewFire_Rifle_Hip_Montage")))))

(fn `AimSlideSmooth`
  (bind _returnvalue (`KismetSystemLibrary.K2_SetTimer` null "AimSlideSmoothTick" (`self.AimStepTimer`) true))
  (set `self.AimTimer` _returnvalue))

(fn `AimSlideSmoothTick`
  (bind _aimchangeslidestepdistance (`self.AimChangeSlideStepDistance`))
  (bind _heightcameramax (`self.HeightCameraMax`))
  (bind _cameraboom (`self.CameraBoom`))
  (bind _targetarmlength (`SpringArmComponent.TargetArmLength` _cameraboom))
  (if (`self.IsAim`)
    (if (< _targetarmlength (+ _heightcameramax (`self.AimDistance`)))
      (set `SpringArmComponent.TargetArmLength` (+ _targetarmlength _aimchangeslidestepdistance) _cameraboom)
      (else
        (`KismetSystemLibrary.K2_ClearAndInvalidateTimerHandle` (`self.AimTimer`) :!label _label)))
    (elif (> _targetarmlength _heightcameramax)
      (set `SpringArmComponent.TargetArmLength` (- _targetarmlength _aimchangeslidestepdistance) _cameraboom)
      (else
        (goto _label)))))

(fn `CameraShakeEvent`
  (`GameplayStatics.PlayWorldCameraShake` "/Game/Blueprints/Game/BP_ShakeCamera.BP_ShakeCamera_C" (`SceneComponent.K2_GetComponentLocation` (`self.TopDownCameraComponent`)) 0.0 30.0))

(fn `CameraSlide`
  (params (Value :type "Float (double-precision)"))
  (bind _heightcamerachangedistance (`self.HeightCameraChangeDistance`))
  (bind _cameraboom (`self.CameraBoom`))
  (bind _targetarmlength (`SpringArmComponent.TargetArmLength` _cameraboom))
  (bind _returnvalue (- _targetarmlength _heightcamerachangedistance))
  (bind _returnvalue_2 (+ _targetarmlength _heightcamerachangedistance))
  (if (!= Value 0.0)
    (if (< Value 0.0)
      (if (>= (`self.HeightCameraMax`) _returnvalue_2)
        (set `SpringArmComponent.TargetArmLength` _returnvalue_2 _cameraboom))
      (elif (<= (`self.HeightCameraMin`) _returnvalue)
        (set `SpringArmComponent.TargetArmLength` _returnvalue _cameraboom)))))

(fn `CameraSlideSmooth`
  (params (Value :type "Float (double-precision)"))
  (bind _heightcamerachangedistance (`self.HeightCameraChangeDistance`))
  (bind _targetarmlength (`SpringArmComponent.TargetArmLength` (`self.CameraBoom`)))
  (if (`self.SlideDone`)
    (if (!= Value 0.0)
      (if (< Value 0.0)
        (if (>= (`self.HeightCameraMax`) (+ _targetarmlength _heightcamerachangedistance))
          (set `self.SlideUp` true)
          (set `self.SlideDone` false :!label _label)
          (bind _returnvalue (`KismetSystemLibrary.K2_SetTimer` null "CameraSlideSmoothTick" (`self.StepTimer`) true))
          (set `self.SlideTimer` _returnvalue))
        (elif (<= (`self.HeightCameraMin`) (- _targetarmlength _heightcamerachangedistance))
          (set `self.SlideUp` false)
          (goto _label))))))

(fn `CameraSlideSmoothTick`
  (bind _heightcamerachangeslidestepdistance (`self.HeightCameraChangeSlideStepDistance`))
  (bind _cameraboom (`self.CameraBoom`))
  (bind _targetarmlength (`SpringArmComponent.TargetArmLength` _cameraboom))
  (bind _output_get (set `self.CurrentSlideDistance` (+ (`self.CurrentSlideDistance`) _heightcamerachangeslidestepdistance)))
  (set `SpringArmComponent.TargetArmLength` (select `bool` (`self.SlideUp`) :`false` (- _targetarmlength _heightcamerachangeslidestepdistance) :`true` (+ _targetarmlength _heightcamerachangeslidestepdistance)) _cameraboom)
  (if (>= _output_get (`self.HeightCameraChangeDistance`))
    (set `self.CurrentSlideDistance` 0.0)
    (set `self.SlideDone` true)
    (`KismetSystemLibrary.K2_ClearAndInvalidateTimerHandle` (`self.SlideTimer`))))

(fn `UserConstructionScript`
  (bind _cameraboom (`self.CameraBoom`))
  (set `SpringArmComponent.TargetArmLength` (`self.HeightCameraMax`) _cameraboom)
  (`SceneComponent.K2_SetRelativeRotation` _cameraboom (`self.RotationCamera`) false false)
  (set `SpringArmComponent.bEnableCameraLag` (`self.Flow`) _cameraboom)
  (set `SpringArmComponent.CameraLagSpeed` (`self.CoefSmooth`) _cameraboom))