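; World ammo pickup that refills one weapon type in the overlapping character's inventory.
; The construction script picks the mesh from WeaponType.
; On character overlap it checks whether the inventory can take that ammo, then adds Cout rounds, plays a type-specific sound and calls PickUpSuccess.
; Tick spins the mesh around yaw by a fixed step per frame, not scaled by delta time.
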(event `self.OnBeginCharacterOverlap`
  (params (Inventory :type "TDSInventoryComponent Object Reference"))
  (bind _weapontype (`self.WeaponType`))
  (`parent.OnBeginCharacterOverlap` Inventory)
  (bind _returnvalue (`TDSInventoryComponent.CheckCanTakeAmmo` Inventory _weapontype))
  (if _returnvalue
    (`TDSInventoryComponent.WeaponChangeAmmo` Inventory _weapontype (`self.Cout`))
    (`GameplayStatics.PlaySoundAtLocation` (select `EWeaponType` _weapontype :`Pistol` "/Game/Items/Game/Weapons/Pistol/Sounds/Pistol_AmmoPickup_Cue.Pistol_AmmoPickup_Cue" :`Rifle` "/Game/Items/Game/Weapons/Rifle/Sounds/Rifle_AmmoPickup_Cue.Rifle_AmmoPickup_Cue" :`SniperRifle` "/Game/Items/Game/Weapons/SniperRifle/Sounds/SniperRifle_AmmoPickup_Cue.SniperRifle_AmmoPickup_Cue" :`Shotgun` "/Game/Items/Game/Weapons/Shotgun/Sounds/Shotgun_AmmoPickup_Cue.Shotgun_AmmoPickup_Cue" :`GrenadeLauncher` "/Game/Items/Game/Weapons/GrenadeLauncher/Sounds/GrenadeLauncher_AmmoPickup_Cue.GrenadeLauncher_AmmoPickup_Cue" :`RocketLauncher` "/Game/Items/Game/Weapons/RocketLauncher/Sounds/RocketLauncher_AmmoPickup_Cue.RocketLauncher_AmmoPickup_Cue" :!type "SoundBase Object Reference") (`self.K2_GetActorLocation` self) (struct) 1.0 1.0 0.0 null null null)
    (`self.PickUpSuccess`)))

(event `self.ReceiveTick`
  (params (DeltaSeconds :type "Float (single-precision)"))
  (bind _staticmesh (`self.StaticMesh`))
  (bind (_returnvalue_roll _returnvalue_pitch _returnvalue_yaw) (`KismetMathLibrary.BreakRotator` (`SceneComponent.K2_GetComponentRotation` _staticmesh)))
  (`parent.ReceiveTick` DeltaSeconds)
  (`/Engine/EditorBlueprintResources/StandardMacros.IsValid` _staticmesh
    (:`Is Valid`
      (`SceneComponent.K2_SetWorldRotation` _staticmesh (`KismetMathLibrary.MakeRotator` _returnvalue_roll _returnvalue_pitch (+ _returnvalue_yaw 0.3)) false false))))

(fn `UserConstructionScript`
  (`parent.UserConstructionScript`)
  (`StaticMeshComponent.SetStaticMesh` (`self.StaticMesh`) (select `EWeaponType` (`self.WeaponType`) :`Pistol` "/Game/Items/Game/Weapons/Pistol/Meshes/Darkness_Pistol_Pickup.Darkness_Pistol_Pickup" :`Rifle` "/Game/Items/Game/Weapons/Rifle/Meshes/Darkness_AssaultRifle_Pickup.Darkness_AssaultRifle_Pickup" :`SniperRifle` "/Game/Items/Game/Weapons/SniperRifle/Meshes/Darkness_SniperRifle_Pickup.Darkness_SniperRifle_Pickup" :`Shotgun` "/Game/Items/Game/Weapons/Shotgun/Meshes/Darkness_Shotgun_Pickup.Darkness_Shotgun_Pickup" :`GrenadeLauncher` "/Game/Items/Game/Weapons/GrenadeLauncher/Meshes/Darkness_GrenadeLauncher_Pickup.Darkness_GrenadeLauncher_Pickup" :`RocketLauncher` "/Game/Items/Game/Weapons/RocketLauncher/Meshes/Darkness_RocketLauncher_Pickup.Darkness_RocketLauncher_Pickup" :!type "StaticMesh Object Reference")))